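; Rubble2_BP is a rubble actor that plays a heavy rock impact sound when its static mesh hits something.
; A short delay after BeginPlay sets Allow, so hits during the first moments of play stay silent.
; Each accepted hit plays the sound at the mesh's location at reduced volume, while the Hit flag and a brief delay act as a cooldown against rapid repeats.
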(event OnComponentHit(StaticMesh)
  (params (HitComponent :type Primitive%20Component%20Object%20Reference) (OtherActor :type Actor%20Object%20Reference) (OtherComp :type Primitive%20Component%20Object%20Reference) (NormalImpulse :type Vector :default "0, 0, 0") (Hit :type Hit%20Result%20Structure%20%28by%20ref%29))
  (if (Variables|Default|GetAllow)
    (if (Variables|Default|GetHit)
      (Variables|Default|SetHit false)
      (Audio|PlaySoundatLocation "/Game/Audio/SFX/PM_RI_Designed_1_Rocks_Impact_Hit_Big_LFE_Heavy_Designed.PM_RI_Designed_1_Rocks_Impact_Hit_Big_LFE_Heavy_Designed" (Transformation|GetWorldLocation (Variables|Default|GetStaticMesh)) "0, 0, 0" 0.3 1.0 0.0 0 0 0)
      (Utilities|FlowControl|Delay 0.7)
      (Variables|Default|SetHit true))))

(event EventBeginPlay
  (Utilities|FlowControl|Delay 2.0)
  (Variables|Default|SetAllow true))

(event Collision|EventActorBeginOverlap
  (params (OtherActor :type Actor%20Object%20Reference)))

(fn ConstructionScript)