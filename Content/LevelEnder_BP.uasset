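; LevelEnder_BP is a Blueprint that shows the level-end report on the HUD.
; Its SetupLevel event loads the game, hides the HUD level timer, then passes rank, trash count, remaining time, last-level flag and win flag to ShowReport.
; A SetHUDRef function supplies the HUD reference it drives.
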(event Custom|Setup%20Level
  (Class|LevelEnder|LoadGame)
  (Widget|SetVisibility (Variables|/Game/Widgets/HUD.HUD_C|GetLevelTimer (Variables|Default|GetHUD)) "Hidden")
  (Default|ShowReport (Variables|Default|GetHUD) (Variables|Default|GetRank) (Variables|Default|GetTrashCount) (Variables|Default|GetTimeRemaining) (Variables|Default|GetOnLastLevel) (Variables|Default|GetWonLevel)))

(fn ConstructionScript)

(fn SetHUDRef
  (params (HUD :type HUD%20Object%20Reference))
  (Variables|Default|SetHUD HUD))