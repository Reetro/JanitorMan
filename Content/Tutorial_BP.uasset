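; Tutorial Blueprint that manages the tutorial's exit menu and the return to the MainMenu level.
; OnLoad hides the level timer on a HUD reference supplied through SetHUD, enables input and creates a hidden BackToMenu widget.
; The Open Exit Menu action uses a FlipFlop to show or hide it, switching cursor and input mode between UI-only and game-only.
; OpenMainMenu removes the widget, restores game input and loads MainMenu.
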(event Custom|On%20Load
  (Widget|SetVisibility (Variables|/Game/Widgets/HUD.HUD_C|GetLevelTimer (Variables|Default|GetHUD)) "Hidden")
  (Input|EnableInput (Game|GetPlayerController 0))
  (bind _returnvalue (UserInterface|CreateWidget "/Game/Widgets/BackToMenu.BackToMenu_C"))
  (bind _output_get (Variables|Default|SetBack%20To%20Main%20Menu _returnvalue))
  (UserInterface|Viewport|AddtoViewport _output_get 0)
  (Widget|SetVisibility (Variables|Default|GetBack%20To%20Main%20Menu) "Hidden"))

(event Custom|Open%20Main%20Menu
  (Widget|RemovefromParent (Variables|Default|GetBack%20To%20Main%20Menu))
  (Variables|/Script/Engine.PlayerController|SetbShowMouseCursor (Game|GetPlayerController 0) false)
  (Variables|/Script/Engine.PlayerController|SetbEnableClickEvents (Game|GetPlayerController 0) false)
  (Variables|/Script/Engine.PlayerController|SetbEnableMouseOverEvents (Game|GetPlayerController 0) false)
  (Input|SetInputModeGameOnly (Game|GetPlayerController 0))
  (Game|OpenLevel(byName) "MainMenu"))

(event Input|ActionEvents|InputActionOpenExitMenu
  (params (Key :type Key%20Structure :default "None"))
  (:Pressed
    (Utilities|FlowControl|FlipFlop
      (:A
        (CallFunction|ShowMenu))
      (:B
        (CallFunction|HideMenu)))))

(fn ConstructionScript)

(fn SetHUD
  (params (HUD :type HUD%20Object%20Reference))
  (Variables|Default|SetHUD HUD))

(fn ShowMenu
  (Variables|/Script/Engine.PlayerController|SetbShowMouseCursor (Game|GetPlayerController 0) true)
  (Variables|/Script/Engine.PlayerController|SetbEnableClickEvents (Game|GetPlayerController 0) true)
  (Variables|/Script/Engine.PlayerController|SetbEnableMouseOverEvents (Game|GetPlayerController 0) true)
  (Variables|/Script/UMG.UserWidget|SetbIsFocusable (Variables|Default|GetBack%20To%20Main%20Menu) true)
  (Input|SetInputModeUIOnly (Game|GetPlayerController 0) (Variables|Default|GetBack%20To%20Main%20Menu) "DoNotLock")
  (Widget|SetVisibility (Variables|Default|GetBack%20To%20Main%20Menu) "Visible"))

(fn HideMenu
  (Widget|SetVisibility (Variables|Default|GetBack%20To%20Main%20Menu) "Hidden")
  (Variables|/Script/Engine.PlayerController|SetbShowMouseCursor (Game|GetPlayerController 0) false)
  (Variables|/Script/Engine.PlayerController|SetbEnableClickEvents (Game|GetPlayerController 0) false)
  (Variables|/Script/Engine.PlayerController|SetbEnableMouseOverEvents (Game|GetPlayerController 0) false)
  (Input|SetInputModeGameOnly (Game|GetPlayerController 0)))