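; Main menu controller Blueprint that shows the menu widget and hands off from the menu into a chosen level.
; OnLoad hides the level timer on the injected HUD, creates and adds the MainMenu widget, and switches the player controller to cursor-driven, UI-only input.
; OpenLevel removes the widget, restores game-only input without the cursor, and loads the given level by name.
; SetHUD supplies the HUD reference.
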(event Custom|On%20Load
  (Widget|SetVisibility (Variables|/Game/Widgets/HUD.HUD_C|GetLevelTimer (Variables|Default|GetHUD)) "Hidden")
  (bind _returnvalue (UserInterface|CreateWidget "/Game/Widgets/MainMenu.MainMenu_C"))
  (bind _output_get (Variables|Default|SetMain%20Menu _returnvalue))
  (UserInterface|Viewport|AddtoViewport _output_get 0)
  (Variables|/Script/Engine.PlayerController|SetbShowMouseCursor (Game|GetPlayerController 0) true)
  (Variables|/Script/Engine.PlayerController|SetbEnableClickEvents (Game|GetPlayerController 0) true)
  (Variables|/Script/Engine.PlayerController|SetbEnableMouseOverEvents (Game|GetPlayerController 0) true)
  (Variables|/Script/UMG.UserWidget|SetbIsFocusable (Variables|Default|GetMain%20Menu) true)
  (Input|SetInputModeUIOnly (Game|GetPlayerController 0) (Variables|Default|GetMain%20Menu) "DoNotLock"))

(event Custom|Open%20Level
  (params (Level%20To%20Open :type Name))
  (Widget|RemovefromParent (Variables|Default|GetMain%20Menu))
  (Variables|/Script/Engine.PlayerController|SetbShowMouseCursor (Game|GetPlayerController 0) false)
  (Variables|/Script/Engine.PlayerController|SetbEnableClickEvents (Game|GetPlayerController 0) false)
  (Variables|/Script/Engine.PlayerController|SetbEnableMouseOverEvents (Game|GetPlayerController 0) false)
  (Input|SetInputModeGameOnly (Game|GetPlayerController 0))
  (Game|OpenLevel(byName) Level%20To%20Open))

(fn ConstructionScript)

(fn SetHUD
  (params (HUD :type HUD%20Object%20Reference))
  (Variables|Default|SetHUD HUD))